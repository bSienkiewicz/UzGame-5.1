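; Weapon helper function library that calculates bullet damage over distance and the delay between shots.
; Damage falloff raises the remaining fraction of max range to a FalloffFactor exponent, without clamping, then applies a small random bonus multiplier.
; Shoot delay converts rounds per minute into seconds per shot and also prints the result as debug output.
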(fn `BFLCalculateWeaponDamageFalloff`
  (params (BulletDamage :type "Float (double-precision)") (MaxRange :type "Float (double-precision)") (Distance :type "Float (double-precision)"))
  (returns (CalculatedDamage :type "Float (double-precision)"))
  (locals (FalloffFactor :type "Float (double-precision)" :default 0.11))
  (return (* (* BulletDamage (`KismetMathLibrary.MultiplyMultiply_FloatFloat` (- 1.0 (/ Distance MaxRange)) (`local.FalloffFactor`))) (`KismetMathLibrary.RandomFloatInRange` 1.0 1.2))))

(fn `BLFCalculateShootDelay`
  (params (RPM :type Integer))
  (returns (Seconds :type "Float (double-precision)"))
  (bind _returnvalue (/ 60.0 (`KismetMathLibrary.Conv_IntToDouble` RPM)))
  (`KismetSystemLibrary.PrintString` null (`KismetStringLibrary.Conv_DoubleToString` _returnvalue))
  (return _returnvalue))