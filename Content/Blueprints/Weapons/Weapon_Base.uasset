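; Base weapon actor for the first-person character, handling pickup, throwing and hitscan shooting, with stubbed fire, reload and ammo hooks.
; Sphere overlap equips it if the player is unarmed, setting the character's WeaponBP child actor class and destroying the pickup.
; Throw spawns an impulse-driven physics copy, passing ammo through the accessors.
; FireHitscan traces from camera with spread, re-traces from muzzle toward that point, and sends damage via BPI_Shootable.
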(event `Equip`
  (params (Ammo :type Integer))
  ;[1 1 1] Equipping the weapon
  (bind _asfirst_person_character (cast `/Game/Blueprints/Player/FirstPersonCharacter` (`GameplayStatics.GetPlayerCharacter` 0)))
  (bind _weapon_bp (`/Game/Blueprints/Player/FirstPersonCharacter.Weapon_BP` _asfirst_person_character))
  (`ChildActorComponent.SetChildActorClass` _weapon_bp (`GameplayStatics.GetObjectClass` self))
  (bind _asweapon_base (cast `/Game/Blueprints/Weapons/Weapon_Base` (`ChildActorComponent.ChildActor` _weapon_bp)))
  (`self.SetAmmoValue` _asweapon_base Ammo))

(event `self.ReceiveBeginPlay`
  ;[1 1 1] GetPlayerRef
  (bind _asfirst_person_character (cast `/Game/Blueprints/Player/FirstPersonCharacter` (`self.GetParentActor`)))
  (set `self.PlayerRef` _asfirst_person_character))

(event `Stow`)

(event `W_Fire`)

(event `Throw`
  ;[1 1 1] Throwing
  (bind _asfirst_person_character (cast `/Game/Blueprints/Player/FirstPersonCharacter` (`GameplayStatics.GetPlayerCharacter` 0)))
  (bind _ammo (`self.GetAmmoValue`))
  (bind _firstpersoncamera (`/Game/Blueprints/Player/FirstPersonCharacter.FirstPersonCamera` _asfirst_person_character))
  (bind _returnvalue (`|SpawnActorFromClass` (`GameplayStatics.GetObjectClass` self) (`KismetMathLibrary.MakeTransform` (+ (`SceneComponent.K2_GetComponentLocation` _firstpersoncamera) (* (`SceneComponent.GetForwardVector` _firstpersoncamera) 100.0)) (`SceneComponent.K2_GetComponentRotation` _firstpersoncamera)) "AdjustIfPossibleButAlwaysSpawn" "OverrideRootScale" null null))
  (`self.SetAmmoValue` _returnvalue _ammo)
  ;;[1 1 1] Throwing
  (bind _asfirst_person_character_2 (cast `/Game/Blueprints/Player/FirstPersonCharacter` (`GameplayStatics.GetPlayerCharacter` 0)))
  (`ChildActorComponent.SetChildActorClass` (`/Game/Blueprints/Player/FirstPersonCharacter.Weapon_BP` _asfirst_person_character_2) null)
  (bind _weapon_mesh (`/Game/Blueprints/Weapons/Weapon_Base.Weapon Mesh` _returnvalue))
  (`PrimitiveComponent.SetSimulatePhysics` _weapon_mesh true)
  (`PrimitiveComponent.SetCollisionProfileName` _weapon_mesh "PhysicsActor" true)
  (`PrimitiveComponent.AddImpulse` _weapon_mesh (* (`SceneComponent.GetForwardVector` _firstpersoncamera) 7000.0) "None" false))

(event `W_StopFiring`)

(event `Reload`)

(event `SetAmmo`)

(event `self.Sphere.OnComponentBeginOverlap`
  (params (OverlappedComponent :type "PrimitiveComponent Object Reference") (OtherActor :type "Actor Object Reference") (OtherComp :type "PrimitiveComponent Object Reference") (OtherBodyIndex :type Integer) (bFromSweep :type Boolean) (SweepResult :type "HitResult Structure (by ref)"))
  (bind _returnvalue (`GameplayStatics.GetPlayerCharacter` 0))
  ;[1 1 1] Equip weapon on overlap
  (if (== OtherActor _returnvalue)
    (`self.GetAmmoValue`)
    (bind _asfirst_person_character (cast `/Game/Blueprints/Player/FirstPersonCharacter` _returnvalue))
    (`/Engine/EditorBlueprintResources/StandardMacros.IsValid` (`/Game/Blueprints/Player/FirstPersonCharacter.GetWeapon` _asfirst_person_character)
      (:`Is Not Valid`
        (bind _ammo (`self.GetAmmoValue`))
        (`KismetSystemLibrary.PrintString` (`KismetStringLibrary.Conv_IntToString` _ammo))
        (`self.Equip` _ammo)
        (`self.K2_DestroyActor`)))))

(fn `Fire_Hitscan`
  (params (DrawDebug :type Boolean) (Spread :type "Float (double-precision)") (Range :type "Float (double-precision)") (Damage :type "Float (double-precision)"))
  (locals (HitInfoL :type "HitResult Structure") (DrawDebug :type Boolean :default true))
  (bind _firstpersoncamera (`/Game/Blueprints/Player/FirstPersonCharacter.FirstPersonCamera` (`self.PlayerRef`)))
  (bind _returnvalue (`SceneComponent.K2_GetComponentLocation` _firstpersoncamera))
  (bind _returnvalue_2 (`KismetMathLibrary.RandomUnitVectorInConeInDegrees` (`SceneComponent.GetForwardVector` _firstpersoncamera) Spread))
  ;[1 1 1] Start Tracing Shoot
  (bind (_outhit _returnvalue_3) (`KismetSystemLibrary.LineTraceSingle` _returnvalue (+ _returnvalue (* _returnvalue_2 Range)) "TraceTypeQuery1" false (`|MakeArray` (`self.PlayerRef`) :!type "Actor Object Reference")))
  ;[1 1 1] Trace From Muzzle To Hit Location
  (set `local.HitInfoL` _outhit)
  (bind (_bblockinghit _binitialoverlap _time _distance _location _impactpoint _normal _impactnormal _physmat _hitactor _hitcomponent _hitbonename _bonename _hititem _elementindex _faceindex _tracestart _traceend) (`GameplayStatics.BreakHitResult` _outhit))
  (bind _outhit_2 (`KismetSystemLibrary.LineTraceSingle` (`SceneComponent.GetSocketLocation` (`self.Weapon Mesh`) "Muzzle") (`KismetMathLibrary.SelectVector` (+ _location (* _returnvalue_2 10.0)) _traceend _returnvalue_3) "TraceTypeQuery1" false (`|MakeArray` (`self.PlayerRef`) :!type "Actor Object Reference") (select `bool` (`local.DrawDebug`) :`true` "ForDuration" :!type "EDrawDebugTrace Enum")))
  (if (`KismetSystemLibrary.DoesImplementInterface` (`.HitActor` (`GameplayStatics.BreakHitResult` _outhit_2)) "/Game/Blueprints/BPI_Shootable.BPI_Shootable_C")
    (message `/Game/Blueprints/BPI_Shootable.GetShot` (`.HitActor` (`GameplayStatics.BreakHitResult` _outhit_2)) Damage)))

(fn `GetAmmoValue`
  (returns (Ammo :type Integer))
  (return 0))

(fn `SetAmmoFromCollided`
  (params (NewWeapon :type "Actor Object Reference") (OvelappedWeapon :type "Actor Object Reference")))

(fn `SetAmmoValue`
  (params (NewAmmoValue :type Integer)))

(fn `ThrowWeapon`
  (params (Camera :type "CameraComponent Object Reference"))
  (bind _returnvalue (`SceneComponent.GetForwardVector` Camera))
  (bind _weapon_mesh (`self.Weapon Mesh`))
  (`PrimitiveComponent.SetSimulatePhysics` _weapon_mesh true)
  (`PrimitiveComponent.SetCollisionProfileName` _weapon_mesh "PhysicsActor" true)
  (`PrimitiveComponent.AddImpulse` _weapon_mesh (+ _returnvalue (* _returnvalue 1000.0)) "None" false))

(fn `UserConstructionScript`)