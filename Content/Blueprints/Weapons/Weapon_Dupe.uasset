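; Full-auto hitscan rifle weapon, built on a parent weapon class, that fires from the player's first-person mesh and shows its ammo on a text component.
; WFire opens a gate that AutoFire re-enters through a timer paced by RoundsPerMinute, until WStopFiring or empty ammo closes it.
; Each shot spends ammo and plays montage, sound and hitscan with debug drawing.
; Reload only plays its montage and toggles IsReloading, without refilling ammo.
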(event `AutoFire`
  ;[1 1 1] Fire Weapon
  ;;[1 1 1] Full Auto Setup
  (`/Engine/EditorBlueprintResources/StandardMacros.Gate` true :!label _label
    (:`Exit`
      (`KismetSystemLibrary.K2_SetTimerDelegate` (delegate `AutoFire`) (stale `self.W_Fire` _seconds) :!label _label_2)
      (if (> (`self.Ammo`) 0)
        ;;[1 1 1] Playing audio and anim
        (set `self.Ammo` (- (`self.Ammo`) 1))
        (`|PlayMontage` (`/Game/Blueprints/Player/FirstPersonCharacter.Mesh_1P` (`self.PlayerRef`)) "/Game/Animations/FIrstPerson/FP_Fire_Montage.FP_Fire_Montage"
          (:`then`
            (`GameplayStatics.PlaySoundAtLocation` "/Game/Audio/Weapons/Rifle/RifleShot_Cue.RifleShot_Cue" (`SceneComponent.K2_GetComponentLocation` (`Character.Mesh` (`GameplayStatics.GetPlayerCharacter` 0))) (struct) 1.0 1.0 0.0 null null null null)
            (`self.Fire_Hitscan` true (`self.Spread`) (`self.Range`) (`self.Damage`))
            (`TextRenderComponent.K2_SetText` (`self.w`) (`KismetTextLibrary.Conv_IntToText` (`self.Ammo`)))))
        (else
          (`|ExecutionSequence`
            (:`then_0`
              (goto _label :!via `Close`))
            (:`then_1`
              (`GameplayStatics.PlaySoundAtLocation` "/Game/Audio/Weapons/Rifle/EmptyClip_Cue.EmptyClip_Cue" (`SceneComponent.K2_GetComponentLocation` (`/Game/Blueprints/Player/FirstPersonCharacter.Mesh_1P` (`self.PlayerRef`))) (struct) 1.0 1.0 0.0 null null null null))))))))

(event `self.W_Fire`
  ;[1 1 1] Fire Weapon
  ;;[1 1 1] Full Auto Setup
  (if (not (`self.isReloading`))
    (`|ExecutionSequence`
      (:`then_0`
        (bind _seconds (`/Game/Blueprints/Weapons/WeaponFunctions.BLFCalculateShootDelay` (`self.RoundsPerMinute`)))
        (goto _label :!via `Open`))
      (:`then_1`
        (goto _label_2)))))

(event `self.W_StopFiring`
  ;[1 1 1] Fire Weapon
  ;;[1 1 1] Full Auto Setup
  (goto _label :!via `Close`))

(event `self.ReceiveTick`
  (params (DeltaSeconds :type "Float (single-precision)"))
  (`TextRenderComponent.K2_SetText` (`self.w`) (`KismetTextLibrary.Conv_IntToText` (`self.Ammo`))))

(event `self.Reload`
  ;[1 0 0.06651] Reload (trash?)
  (if (not (`self.isReloading`))
    (set `self.isReloading` true)
    (`|PlayMontage` (`/Game/Blueprints/Player/FirstPersonCharacter.Mesh_1P` (`self.PlayerRef`)) "/Game/Animations/FIrstPerson/FP_Reload_Montage.FP_Reload_Montage"
      (:`OnBlendOut`
        (set `self.isReloading` false))
      (:`OnInterrupted`
        (`KismetSystemLibrary.Delay` 0.2)
        (set `self.isReloading` true)))))

(event `/Game/Blueprints/Weapons/BPI_Weapons.SetWeaponAmmoValue`
  (params (Ammo :type Integer)))

(fn `GetAmmoValue`
  (returns (Ammo :type Integer))
  (`parent.GetAmmoValue`)
  (return (`self.Ammo`)))

(fn `GetWeaponAmmoValue`
  (returns (Ammo :type Integer))
  (return (`self.Ammo`)))

(fn `SetAmmoOnPickup`
  (params (Ammo :type Integer))
  (set `self.Ammo` Ammo))

(fn `SetAmmoValue`
  (params (NewAmmoValue :type Integer))
  (`parent.SetAmmoValue` 0)
  (set `self.Ammo` NewAmmoValue))

(fn `UserConstructionScript`
  (`parent.UserConstructionScript`)
  (`TextRenderComponent.K2_SetText` (`self.w`) (`KismetTextLibrary.Conv_IntToText` (`self.Ammo`))))