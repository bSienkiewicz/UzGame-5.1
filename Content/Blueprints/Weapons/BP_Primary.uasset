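; Primary weapon Blueprint that the player equips on interact and fires as a fully automatic hitscan gun.
; Shoot opens a gate and fires at once, then a timer delayed from the weapon's RPM re-enters the gate until StopShooting closes it.
; Each shot spends ammo, line-traces from the camera, spawns an impact emitter and passes distance-falloff damage to BPI_Shootable actors.
; An empty magazine only prints a message.
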(event `/Game/Blueprints/BPI_Interactable.Interact`
  (params (Player :type "Actor Object Reference"))
  (bind _asfirst_person_character (cast `/Game/Blueprints/Player/FirstPersonCharacter` Player))
  (`/Game/Blueprints/Player/FirstPersonCharacter.EquipNewWeapon` _asfirst_person_character self))

(event `AutoFire`
  (bind (_weaponstats_bulletdamage _weaponstats_range) (break `/Game/Blueprints/Weapons/STR_WeaponStats` (`self.WeaponStats`)))
  (bind (_weaponstats_bulletdamage_2 _weaponstats_range_2 _weaponstats_rpm _weaponstats_magsize) (break `/Game/Blueprints/Weapons/STR_WeaponStats` (`self.WeaponStats`)))
  ;[1 1 1] Shooting hitscan
  (`/Engine/EditorBlueprintResources/StandardMacros.Gate` true :!label _label
    (:`Exit`
      (`KismetSystemLibrary.K2_SetTimerDelegate` (delegate `AutoFire`) (stale `/Game/Blueprints/Weapons/BPI_Weapons.Shoot` _seconds) :!label _label_2)
      (if (<= _weaponstats_magsize 0)
        (`KismetSystemLibrary.PrintString` "NoAmmo")
        (else
          (set `self.WeaponStats` (make `/Game/Blueprints/Weapons/STR_WeaponStats` _weaponstats_bulletdamage_2 _weaponstats_range_2 _weaponstats_rpm (- _weaponstats_magsize 1)))
          (bind _returnvalue (`SceneComponent.K2_GetComponentLocation` (stale `/Game/Blueprints/Weapons/BPI_Weapons.Shoot` Camera)))
          (bind _outhit (`KismetSystemLibrary.LineTraceSingle` :`Start` _returnvalue :`End` (+ _returnvalue (* (`KismetMathLibrary.GetForwardVector` (`SceneComponent.K2_GetComponentRotation` (stale `/Game/Blueprints/Weapons/BPI_Weapons.Shoot` Camera))) _weaponstats_range_2)) :`TraceChannel` "TraceTypeQuery1" :`DrawDebugType` "ForDuration" :`TraceColor` (struct :`G` 0.002356 :`B` 1.0 :`A` 1.0)))
          (`GameplayStatics.SpawnEmitterAtLocation` null (`.Location` (`GameplayStatics.BreakHitResult` _outhit)) (struct) (0.5 0.5 0.5))
          (if (`KismetSystemLibrary.DoesImplementInterface` (`.HitActor` (`GameplayStatics.BreakHitResult` _outhit)) "/Game/Blueprints/BPI_Shootable.BPI_Shootable_C")
            (bind _asbpi_shootable (cast `/Game/Blueprints/BPI_Shootable` (`.HitActor` (`GameplayStatics.BreakHitResult` _outhit))))
            (bind _calculateddamage (`/Game/Blueprints/Weapons/WeaponFunctions.BFLCalculateWeaponDamageFalloff` _weaponstats_bulletdamage _weaponstats_range (`.Distance` (`GameplayStatics.BreakHitResult` _outhit))))
            (`/Game/Blueprints/BPI_Shootable.GetShot` _asbpi_shootable _calculateddamage)))))))

(event `/Game/Blueprints/Weapons/BPI_Weapons.StopShooting`
  ;[1 1 1] Shooting hitscan
  (goto _label :!via `Close`))

(event `/Game/Blueprints/Weapons/BPI_Weapons.Shoot`
  (params (Camera :type "CameraComponent Object Reference"))
  (bind (_weaponstats_bulletdamage _weaponstats_range _weaponstats_rpm _weaponstats_magsize) (break `/Game/Blueprints/Weapons/STR_WeaponStats` (`self.WeaponStats`)))
  ;[1 1 1] Shooting hitscan
  (`KismetSystemLibrary.PrintString` (`KismetStringLibrary.Conv_IntToString` _weaponstats_magsize))
  (bind _seconds (`/Game/Blueprints/Weapons/WeaponFunctions.BLFCalculateShootDelay` _weaponstats_rpm))
  (`|ExecutionSequence`
    (:`then_0`
      (goto _label :!via `Open`))
    (:`then_1`
      (goto _label_2))))

(fn `NewFunction`)

(fn `UserConstructionScript`)