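; Test enemy pawn that spots the first-person player and performs a placeholder melee attack.
; PawnSensing sets the HasSeenPlayer blackboard key on its AI controller when it sees a FirstPersonCharacter.
; AttackPlayer runs a short forward sphere trace against pawns and only prints a debug message when the first hit is the player, without applying damage.
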(event `self.PawnSensing.OnSeePawn`
  (params (Pawn :type "Pawn Object Reference"))
  (cast `/Game/Blueprints/Player/FirstPersonCharacter` Pawn)
  (`BlackboardComponent.SetValueAsBool` (`AIBlueprintHelperLibrary.GetBlackboard` (`AIBlueprintHelperLibrary.GetAIController` self)) "HasSeenPlayer" true))

(event `AttackPlayer`
  (bind _returnvalue (`self.K2_GetActorLocation`))
  (bind (_outhit _returnvalue_2) (`KismetSystemLibrary.SphereTraceSingleForObjects` :`Start` _returnvalue :`End` (+ _returnvalue (* (`KismetMathLibrary.GetForwardVector` (`self.K2_GetActorRotation`)) 250.0)) :`Radius` 120.0 :`ObjectTypes` (`|MakeArray` "ObjectTypeQuery3" :!type "EObjectTypeQuery Enum") :`DrawDebugType` "ForDuration"))
  (if _returnvalue_2
    (cast `/Game/Blueprints/Player/FirstPersonCharacter` (`.HitActor` (`GameplayStatics.BreakHitResult` _outhit)))
    (`KismetSystemLibrary.PrintString` "ATTACKING PLAYER" true true (struct :`R` 1.0 :`B` 0.104458 :`A` 1.0))))

(fn `UserConstructionScript`)