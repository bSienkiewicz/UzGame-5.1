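; BP_PrimaryRed is an equippable hitscan weapon that the first-person character takes through Interact.
; Shoot runs a debug-drawn visibility line trace scaled by weapon range, with location and rotation inputs left at zero rather than taken from the player or muzzle.
; It spawns an explosion effect at the hit location and passes fixed damage to hit actors implementing BPI_Shootable through GetShot.
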(event `/Game/Blueprints/BPI_Interactable.Interact`
  (params (Player :type "Actor Object Reference"))
  (bind _asfirst_person_character (cast `/Game/Blueprints/Player/FirstPersonCharacter` Player))
  (`/Game/Blueprints/Player/FirstPersonCharacter.EquipNewWeapon` _asfirst_person_character self))

(event `/Game/Blueprints/Weapons/BPI_Weapons.Shoot`
  (params (Camera :type "CameraComponent Object Reference"))
  (bind (_weaponstats_bulletdamage _weaponstats_range) (break `/Game/Blueprints/Weapons/STR_WeaponStats` (`self.WeaponStats`)))
  ;[1 1 1] Shooting hitscan
  (bind _outhit (`KismetSystemLibrary.LineTraceSingle` :`End` (+ (0.0 0.0 0.0) (* (`KismetMathLibrary.GetForwardVector` (struct)) _weaponstats_range)) :`TraceChannel` "TraceTypeQuery1" :`DrawDebugType` "ForDuration" :`TraceColor` (struct :`R` 1.0 :`B` 0.743414 :`A` 1.0)))
  (`GameplayStatics.SpawnEmitterAtLocation` "/Game/StarterContent/Particles/P_Explosion.P_Explosion" (`.Location` (`GameplayStatics.BreakHitResult` _outhit)) (struct) (0.5 0.5 0.5))
  (if (`KismetSystemLibrary.DoesImplementInterface` (`.HitActor` (`GameplayStatics.BreakHitResult` _outhit)) "/Game/Blueprints/BPI_Shootable.BPI_Shootable_C")
    (bind _asbpi_shootable (cast `/Game/Blueprints/BPI_Shootable` (`.HitActor` (`GameplayStatics.BreakHitResult` _outhit))))
    (`/Game/Blueprints/BPI_Shootable.GetShot` _asbpi_shootable 30.0)))

(fn `NewFunction`)

(fn `UserConstructionScript`)