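; BP_Target is a shootable target actor that loses health when hit by weapon fire.
; GetShot prints the incoming WeaponDamage and subtracts it from Stats.Health, rebuilding the struct with its other fields zeroed.
; Die spawns a scaled-up explosion at the capsule and destroys the actor.
; The zero-health branch is empty and the only Die call is disconnected, so this graph never triggers death.
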(event `/Game/Blueprints/BPI_Shootable.GetShot`
  (params (`Weapon Damage` :type "Float (double-precision)"))
  (bind _stats_health (break `/Game/Blueprints/STR_EnemyStats` (`self.Stats`)))
  (`KismetSystemLibrary.PrintString` (`KismetStringLibrary.Conv_DoubleToString` `Weapon Damage`))
  (bind _output_get (set `self.Stats` (make `/Game/Blueprints/STR_EnemyStats` (- _stats_health `Weapon Damage`))))
  (if (<= (break `/Game/Blueprints/STR_EnemyStats` _output_get) 0.0)
    _))

(event `Die`
  (`GameplayStatics.SpawnEmitterAtLocation` "/Game/StarterContent/Particles/P_Explosion.P_Explosion" (`SceneComponent.K2_GetComponentLocation` (`self.CapsuleComponent`)) (struct) (3.0 3.0 3.0))
  (`self.K2_DestroyActor`))

(fn `UserConstructionScript`)