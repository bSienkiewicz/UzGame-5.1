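; BP_Door is a swinging door that opens when the player character enters its collision volume.
; A timeline drives the door mesh's yaw on overlap and reverses on any actor's end overlap, with IsClosed tracking the state.
; The Kick event is empty; a second timeline for a one-shot open that changes the collision profile, and a DoorClosing call, are left disconnected.
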(event `self.Collision.OnComponentBeginOverlap`
  (params (OverlappedComponent :type "PrimitiveComponent Object Reference") (OtherActor :type "Actor Object Reference") (OtherComp :type "PrimitiveComponent Object Reference") (OtherBodyIndex :type Integer) (bFromSweep :type Boolean) (SweepResult :type "HitResult Structure (by ref)"))
  (if (== OtherActor (`GameplayStatics.GetPlayerCharacter` 0))
    (set `self.isClosed` false)
    (bind (_direction _rotation) (`Timeline|Timeline` :!label _label)
      (:`Update`
        (`SceneComponent.K2_SetRelativeRotation` (`self.SM_Door`) (`KismetMathLibrary.MakeRotator` 0.0 0.0 _rotation) false false)))))

(event `self.Collision.OnComponentEndOverlap`
  (params (OverlappedComponent :type "PrimitiveComponent Object Reference") (OtherActor :type "Actor Object Reference") (OtherComp :type "PrimitiveComponent Object Reference") (OtherBodyIndex :type Integer))
  (if true
    (set `self.isClosed` true)
    (goto _label :!via `Reverse`)))

(event `/Game/Blueprints/I_Kickable.Kick`)

(fn `UserConstructionScript`)