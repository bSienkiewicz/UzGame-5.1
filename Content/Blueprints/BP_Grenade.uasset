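; Grenade actor that ticks audibly, shows a screen-space widget over itself, and explodes once it slows down.
; SpawnGrenade starts the sound and widget; Tick projects the sphere's position to move the widget and calls Explode at low speed.
; Explode raises the ticking pitch, waits, spawns particles, applies radial impulse, then prints overlapped actor names and destroys itself within that loop.
; Destruction removes the widget and plays the explosion sound.
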(event `SpawnGrenade`
  ;[0 0.1238 1] Spawn
  (bind _returnvalue (`GameplayStatics.SpawnSoundAttached` "/Game/Audio/Weapons/Ticking_Cue.Ticking_Cue" (`self.Sphere`) "None" (0.0 0.0 0.0) (struct) "KeepWorldPosition" true 0.5 1.0 0.0 null null))
  (set `self.TickingSound` _returnvalue)
  (bind _returnvalue_2 (`|CreateWidget` "/Game/Blueprints/WUI_Test.WUI_Test_C" (`GameplayStatics.GetPlayerController` 0)))
  (bind _output_get (set `self.Widget` _returnvalue_2))
  (`UserWidget.AddToViewport` _output_get 0))

(event `self.ReceiveDestroyed`
  ;[1 1 1] On Destroy
  (`Widget.RemoveFromParent` (stale `SpawnGrenade` _returnvalue_2))
  (`GameplayStatics.PlaySoundAtLocation` "/Game/StarterContent/Audio/Explosion02.Explosion02" (`SceneComponent.K2_GetComponentLocation` (`self.Sphere`)) (struct) 1.0 1.0 0.0 null null null null))

(event `self.Explode`
  (bind _tickingsound (`self.TickingSound`))
  (bind _sphere (`self.Sphere`))
  (bind _returnvalue (`SceneComponent.K2_GetComponentLocation` _sphere))
  ;[1 0.1678 0] Explode
  (`/Engine/EditorBlueprintResources/StandardMacros.IsValid` _tickingsound
    (:`Is Valid`
      (`AudioComponent.SetPitchMultiplier` _tickingsound 1.4)
      (`KismetSystemLibrary.Delay` 1.0)
      (`GameplayStatics.SpawnEmitterAtLocation` "/Game/StarterContent/Particles/P_Explosion.P_Explosion" _returnvalue (struct) (3.0 3.0 3.0))
      (`PrimitiveComponent.AddRadialImpulse` _sphere _returnvalue 500.0 10000.0 "RIF_Constant" false)
      (bind _outactors (`KismetSystemLibrary.SphereOverlapActors` _returnvalue 500.0 (`|MakeArray` "ObjectTypeQuery3" "ObjectTypeQuery1" :!type "EObjectTypeQuery Enum")))
      (for _array_element _outactors
        (`KismetSystemLibrary.PrintString` (`KismetSystemLibrary.GetDisplayName` _array_element))
        (`self.K2_DestroyActor`)))))

(event `self.ReceiveTick`
  (params (DeltaSeconds :type "Float (single-precision)"))
  ;[1 1 1] Tick
  (`UserWidget.SetPositionInViewport` (`self.Widget`) (`GameplayStatics.ProjectWorldToScreen` (`GameplayStatics.GetPlayerController` 0) (`SceneComponent.K2_GetComponentLocation` (`self.Sphere`))) true)
  (if (<= (`KismetMathLibrary.VSize` (`self.GetVelocity`)) 100.0)
    (`self.Explode`)))

(fn `UserConstructionScript`)